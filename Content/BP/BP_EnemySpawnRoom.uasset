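; A room actor that spawns enemies or health pickups, or serves as the final room that ends the level.
; On BeginPlay the server scales the room, randomizes non-final types and spawns an initial batch at random interior points.
; While a character overlaps, Tick plus Delay repeats spawning until projectile hits deplete spawner health, destroying the room actor.
; Final rooms count overlaps, showing a completion widget and pausing when matching the player-controller count.
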(event `Change Player COunt`
  (params (NewParam :type Integer))
  (bind _output_get (set `self.numOfPLayersInRoom` (+ (`self.numOfPLayersInRoom`) NewParam)))
  (if (== (`GameplayStatics.GetNumPlayerControllers`) _output_get)
    (`self.End game`)))

(event `End game`
  (bind _returnvalue (`GameplayStatics.GetPlayerController` 0))
  (bind _returnvalue_2 (`|CreateWidget` "/Game/BP/UIStuff/W_LevelComplete.W_LevelComplete_C"))
  (`UserWidget.AddToViewport` _returnvalue_2 0)
  (`GameplayStatics.SetGamePaused` true)
  (`WidgetBlueprintLibrary.SetInputMode_UIOnlyEx` _returnvalue null)
  (set `PlayerController.bShowMouseCursor` true _returnvalue))

(event `self.ReceiveBeginPlay`
  (bind _returnvalue (`KismetMathLibrary.RandomIntegerInRange` 1 5))
  (bind _returnvalue_2 (`KismetMathLibrary.RandomInteger` 5))
  (`/Engine/EditorBlueprintResources/ActorMacros.Switch Has Authority`
    (:`Authority`
      (`self.SetRoomSize`)
      (switch `int` (`self.RoomType`)
        (:`Default`
          ;[1 1 1] Room Type: Enemy
          (for _ (range (+ _returnvalue 1)) :!label _label
            (`self.SpawnRandomEnemyType`))
          (`KismetSystemLibrary.PrintString` (`KismetStringLibrary.Concat_StrStr` (`KismetStringLibrary.Concat_StrStr` (`KismetStringLibrary.Conv_IntToString` _returnvalue) " Enemies spawned in room: ") (`KismetSystemLibrary.GetDisplayName` self))))
        (:`0`
          (goto _label))
        (:`1`
          ;[1 1 1] Room Type: Health Pickup
          (for _ (range (+ _returnvalue_2 1))
            (`self.SpawnHealthPickup`))
          (`KismetSystemLibrary.PrintString` (`KismetStringLibrary.Concat_StrStr` (`KismetStringLibrary.Concat_StrStr` (`KismetStringLibrary.Conv_IntToString` _returnvalue_2) " Health pickups spawned in room: ") (`KismetSystemLibrary.GetDisplayName` self))))
        (:`2`
          (set `self.isFinalRoom` true)
          (`SceneComponent.SetVisibility` (`self.Spawner`) false false))))))

(event `Deactivate`
  (set `self.IsActive` false))

(event `Activate`
  (set `self.IsActive` true))

(event `self.RoomInterior.OnComponentBeginOverlap`
  (params (OverlappedComponent :type "PrimitiveComponent Object Reference") (OtherActor :type "Actor Object Reference") (OtherComp :type "PrimitiveComponent Object Reference") (OtherBodyIndex :type Integer) (bFromSweep :type Boolean) (SweepResult :type "HitResult Structure (by ref)"))
  (if (`self.isFinalRoom`)
    (`self.Change Player COunt` 1)
    (else
      (`/Engine/EditorBlueprintResources/ActorMacros.Switch Has Authority`
        (:`Authority`
          (cast `/Game/ThirdPerson/Blueprints/BP_ThirdPersonCharacter` OtherActor)
          (`self.Activate`))))))

(event `self.ReceiveTick`
  (params (DeltaSeconds :type "Float (single-precision)"))
  (`/Engine/EditorBlueprintResources/ActorMacros.Switch Has Authority`
    (:`Authority`
      (if (`self.IsActive`)
        (`KismetSystemLibrary.Delay` (`self.SpawnTime`))
        (switch `int` (`self.RoomType`)
          (:`Default`
            (`self.SpawnRandomEnemyType` :!label _label_2))
          (:`0`
            (goto _label_2))
          (:`1`
            (`self.SpawnHealthPickup`)))))))

(event `self.RoomInterior.OnComponentEndOverlap`
  (params (OverlappedComponent :type "PrimitiveComponent Object Reference") (OtherActor :type "Actor Object Reference") (OtherComp :type "PrimitiveComponent Object Reference") (OtherBodyIndex :type Integer))
  (if (`self.isFinalRoom`)
    (`self.Change Player COunt` -1)
    (else
      (`/Engine/EditorBlueprintResources/ActorMacros.Switch Has Authority`
        (:`Authority`
          (cast `/Game/ThirdPerson/Blueprints/BP_ThirdPersonCharacter` OtherActor)
          (`self.Deactivate`))))))

(event `Hit`
  (params (DAmage :type "Float (double-precision)") (Object :type "/Game/FirstPerson/Blueprints/BP_FirstPersonProjectile Object Reference"))
  (`self.K2_DestroyActor` (stale `/Game/BP/I_Interact.OnHit` Object))
  (`self.K2_DestroyActor` Object)
  (bind _output_get (set `self.SpawnerHealth` (- (`self.SpawnerHealth`) DAmage)))
  (`KismetSystemLibrary.PrintString` (`KismetStringLibrary.Conv_DoubleToString` _output_get))
  (if (<= _output_get 0.0)
    (`self.K2_DestroyActor`)))

(event `/Game/BP/I_Interact.OnHit`
  (params (Damage :type "Float (double-precision)") (Object :type "/Game/FirstPerson/Blueprints/BP_FirstPersonProjectile Object Reference"))
  (`self.Hit` Damage Object))

(event `self.Spawner.OnComponentHit`
  (params (HitComponent :type "PrimitiveComponent Object Reference") (OtherActor :type "Actor Object Reference") (OtherComp :type "PrimitiveComponent Object Reference") (NormalImpulse :type "Vector Structure") (Hit :type "HitResult Structure (by ref)"))
  (`/Engine/EditorBlueprintResources/ActorMacros.Switch Has Authority`
    (:`Authority`
      (bind _asbp_first_person_projectile (cast `/Game/FirstPerson/Blueprints/BP_FirstPersonProjectile` OtherActor))
      (`KismetSystemLibrary.PrintString` "oBJECT HIT")
      (bind _output_get (set `self.SpawnerHealth` (- (`self.SpawnerHealth`) (`/Game/FirstPerson/Blueprints/BP_FirstPersonProjectile.Damage` _asbp_first_person_projectile))))
      (`self.K2_DestroyActor` _asbp_first_person_projectile)
      (`KismetSystemLibrary.PrintString` (`KismetStringLibrary.Conv_DoubleToString` _output_get))
      (if (<= _output_get 0.0)
        (`self.K2_DestroyActor`)))))

(event `SpawnRandomEnemyType`
  (bind (_origin _boxextent) (`KismetSystemLibrary.GetComponentBounds` (`self.RoomInterior`)))
  (bind _returnvalue (`KismetMathLibrary.Conv_VectorToTransform` (`KismetMathLibrary.RandomPointInBoundingBox` _origin _boxextent)))
  (`/Engine/EditorBlueprintResources/ActorMacros.Switch Has Authority`
    (:`Authority`
      (bind _returnvalue_2 (`|SpawnActorFromClass` "/Game/BP/BP_EnemyAI.BP_EnemyAI_C" (`KismetMathLibrary.MakeTransform` (`KismetMathLibrary.MakeVector` (.x (.location _returnvalue)) (.y (.location _returnvalue)) 1.0) (`KismetMathLibrary.MakeRotator` 0.0 0.0 (`KismetMathLibrary.RandomFloatInRange` 0.0 180.0))) "Undefined" "MultiplyWithRoot" null null))
      (`KismetSystemLibrary.Delay` 0.5)
      (if (== (`KismetMathLibrary.RandomIntegerInRange` 1 2) 1)
        (set `/Game/BP/BP_EnemyAI.Ranged?` true _returnvalue_2)
        (`/Game/BP/BP_EnemyAI.Set Enemy Type` _returnvalue_2)))))

(event `SpawnHealthPickup`
  (bind (_origin _boxextent) (`KismetSystemLibrary.GetComponentBounds` (`self.RoomInterior`)))
  (`/Engine/EditorBlueprintResources/ActorMacros.Switch Has Authority`
    (:`Authority`
      (`|SpawnActorFromClass` "/Game/BP/BP_HealthPickup.BP_HealthPickup_C" (`KismetMathLibrary.MakeTransform` (`KismetMathLibrary.RandomPointInBoundingBox` _origin _boxextent) (struct) (0.5 0.5 0.5)) "AdjustIfPossibleButAlwaysSpawn" "MultiplyWithRoot" null null)
      (`KismetSystemLibrary.PrintString` "Hello"))))

(fn `IsInteractable`
  (returns (isInteractable :type Boolean))
  (return false))

(fn `SetRoomSize`
  (`SceneComponent.SetRelativeScale3D` (`self.RoomInterior`) (`self.RoomDimensions`))
  (if (!= (`self.RoomType`) 2)
    (if (>= (`KismetMathLibrary.RandomIntegerInRange` 1 100) 80)
      (set `self.RoomType` 1)
      (else
        (set `self.RoomType` 0)))))

(fn `UserConstructionScript`)