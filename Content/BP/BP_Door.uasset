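; BP_Door is an interactable door that swings open or closed when a character uses it.
; OnInteract passes through server and multicast events, which toggle IsOpen and play or reverse a Timeline driving the mesh's yaw.
; On opening, swing direction comes from dotting the root-to-character direction with the root's world location, not a facing vector.
; Box overlap logic for CanInteract is disconnected, and OnHit and OnRep are empty.
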(event `self.Box.OnComponentBeginOverlap`
  (params (OverlappedComponent :type "PrimitiveComponent Object Reference") (OtherActor :type "Actor Object Reference") (OtherComp :type "PrimitiveComponent Object Reference") (OtherBodyIndex :type Integer) (bFromSweep :type Boolean) (SweepResult :type "HitResult Structure (by ref)")))

(event `self.Box.OnComponentEndOverlap`
  (params (OverlappedComponent :type "PrimitiveComponent Object Reference") (OtherActor :type "Actor Object Reference") (OtherComp :type "PrimitiveComponent Object Reference") (OtherBodyIndex :type Integer)))

(event `/Game/BP/I_Interact.OnInteract`
  (params (Character :type "Character Object Reference"))
  (`self.Server_OpenDoor` Character))

(event `Server_OpenDoor`
  (params (Character :type "Character Object Reference"))
  (`self.Multicast_Open_Door` Character))

(event `Multicast_Open_Door`
  (params (Character :type "Character Object Reference"))
  (bind _returnvalue (`SceneComponent.K2_GetComponentLocation` (`self.DefaultSceneRoot`)))
  (if (`self.isOpen`)
    (set `self.isOpen` false)
    (bind (_direction _dooropen) (`Timeline|Timeline` :!via `Reverse` :!label _label)
      (:`Update`
        (`SceneComponent.K2_SetRelativeRotation` (`self.StaticMesh`) (`KismetMathLibrary.MakeRotator` 0.0 90.0 (* _dooropen (stale _output_get))) false false)))
    (else
      (set `self.isOpen` true)
      (bind _output_get (set `self.endRotation` (`KismetMathLibrary.SelectFloat` 90.0 -90.0 (>= (`KismetMathLibrary.Dot_VectorVector` (`KismetMathLibrary.Normal` (- (`self.K2_GetActorLocation` Character) _returnvalue)) _returnvalue) 0.0))))
      (goto _label))))

(fn `IsInteractable`
  (returns (isInteractable :type Boolean))
  (return (`self.canInteract`)))

(fn `OnHit`
  (params (Damage :type "Float (double-precision)") (Object :type "/Game/FirstPerson/Blueprints/BP_FirstPersonProjectile Object Reference"))
  (return))

(fn `OnRep_isOpen`)

(fn `UserConstructionScript`)