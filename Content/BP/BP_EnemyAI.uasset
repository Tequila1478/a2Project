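; Enemy AI pawn that chases and attacks the third-person player as either a melee or ranged type, with the Ranged flag choosing the visible weapon at construction.
; PawnSensing triggers an AIMoveTo follow-and-attack loop with randomised delays and timer-driven turning toward the player.
; Melee damage requires player overlap with a hit box, while ranged attacks fire the weapon component.
; RagDollOnHit handles death; state events are empty stubs.
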(event `SwitchState`
  (params (NewState :type Integer)))

(event `StateIdle`)

(event `StateFollow`)

(event `StateAttack`)

(event `self.ReceiveBeginPlay`)

(event `self.PawnSensing.OnSeePawn`
  (params (Pawn :type "Pawn Object Reference"))
  (set `self.CanSeePlayer?` true)
  (bind _asbp_third_person_character (cast `/Game/ThirdPerson/Blueprints/BP_ThirdPersonCharacter` Pawn))
  (set `self.Player` _asbp_third_person_character)
  (if (`self.Ranged?`)
    (`self.FollowPlayer_Ranged`)
    (else
      (`self.FollowPlayer_Melee`))))

(event `FollowPlayer_Ranged`
  (if (`self.CanSeePlayer?`)
    (set `self.isMoving` true)
    (`|AIMoveTo` self (0.0 0.0 0.0) (`self.Player`) 400.0
      (:`OnSuccess`
        (if (`self.CanAttack`)
          (`self.ShootPlayer`)
          (set `self.isMoving` false)
          (`self.FollowPlayer_Ranged`))))))

(event `FollowPlayer_Melee`
  (if (`self.CanSeePlayer?`)
    (set `self.isMoving` true)
    (`|AIMoveTo` self (0.0 0.0 0.0) (`self.Player`) 150.0
      (:`OnSuccess`
        (if (`self.CanAttack`)
          (`self.AttackPlayer`)
          (set `self.isMoving` false)
          (`self.FollowPlayer_Melee`))))))

(event `AttackPlayer`
  (`KismetSystemLibrary.K2_SetTimerDelegate` (delegate `RotateAI`) 0.01 true true)
  (set `self.CanAttack` false)
  (`KismetSystemLibrary.Delay` (+ (* (`KismetMathLibrary.RandomFloat`) 2.0) 0.5))
  (`self.PlayAnimMontage` "/Game/Sword_Animation/Animations/anim_attack_light_01_Montage.anim_attack_light_01_Montage" 1.0 (`KismetStringLibrary.Conv_StringToName` (`|GetArrayItem` (`self.LightAttacks`) (`KismetMathLibrary.RandomInteger` 2))))
  (if (`self.canHitPlayer`)
    (message `/Game/BP/I_Interact.OnHit` (`self.Player`) 10.0 null))
  (set `self.CanAttack` true))

(event `ShootPlayer`
  (if (not (`self.isDead`))
    (`KismetSystemLibrary.K2_SetTimerDelegate` (delegate `RotateAI`) 0.01 true true)
    (set `self.CanAttack` false)
    (`KismetSystemLibrary.Delay` (* (`KismetMathLibrary.RandomFloat`) 2.0))
    (`self.PlayAnimMontage` "/Game/AnimStarterPack/UE5_Upgraded/Fire_Rifle_Hip_Montage.Fire_Rifle_Hip_Montage" 1.0 "Default")
    (`KismetSystemLibrary.Delay` 0.2)
    (`/Game/FirstPerson/Blueprints/BP_Weapon_Component_Enemy.FireGun` (`self.WC_Ranged`))
    (set `self.CanAttack` true)))

(event `RotateAI`
  (bind (_returnvalue_roll _returnvalue_pitch _returnvalue_yaw) (`KismetMathLibrary.BreakRotator` (`KismetMathLibrary.FindLookAtRotation` (`self.K2_GetActorLocation`) (`self.K2_GetActorLocation` (`self.Player`)))))
  (`self.K2_SetActorRotation` (`KismetMathLibrary.RInterpTo` (`self.K2_GetActorRotation`) (`KismetMathLibrary.MakeRotator` 0.0 0.0 _returnvalue_yaw) (`GameplayStatics.GetWorldDeltaSeconds`) 1.0)))

(event `CheckIfPlayerCanBeHit`
  (bind _returnvalue (`self.K2_GetActorRotation`))
  (bind _returnvalue_2 (`KismetMathLibrary.Vector_Normal2D` (- (`self.K2_GetActorLocation` (`GameplayStatics.GetPlayerController` 0)) (`self.K2_GetActorLocation`))))
  (`KismetSystemLibrary.PrintString` (`KismetStringLibrary.Conv_DoubleToString` (`KismetMathLibrary.DegAtan2` (`KismetMathLibrary.Dot_VectorVector` _returnvalue_2 (`KismetMathLibrary.Vector_Normal2D` (`KismetMathLibrary.GetRightVector` _returnvalue))) (`KismetMathLibrary.Dot_VectorVector` _returnvalue_2 (`KismetMathLibrary.Vector_Normal2D` (`KismetMathLibrary.GetForwardVector` _returnvalue)))))))

(event `self.Box.OnComponentBeginOverlap`
  (params (OverlappedComponent :type "PrimitiveComponent Object Reference") (OtherActor :type "Actor Object Reference") (OtherComp :type "PrimitiveComponent Object Reference") (OtherBodyIndex :type Integer) (bFromSweep :type Boolean) (SweepResult :type "HitResult Structure (by ref)"))
  (cast `/Game/ThirdPerson/Blueprints/BP_ThirdPersonCharacter` OtherActor)
  (set `self.canHitPlayer` true))

(event `self.Box.OnComponentEndOverlap`
  (params (OverlappedComponent :type "PrimitiveComponent Object Reference") (OtherActor :type "Actor Object Reference") (OtherComp :type "PrimitiveComponent Object Reference") (OtherBodyIndex :type Integer))
  (cast `/Game/ThirdPerson/Blueprints/BP_ThirdPersonCharacter` OtherActor)
  (set `self.canHitPlayer` false))

(event `Set Enemy Type`
  (bind _wc_ranged (`self.WC_Ranged`))
  (if (`self.Ranged?`)
    (`SceneComponent.SetVisibility` (`self.WC_Melee`) false true)
    (`SceneComponent.SetVisibility` _wc_ranged true true)
    (set `/Game/FirstPerson/Blueprints/BP_Weapon_Component_Enemy.ProjectileOffset` (50.0 30.0 0.0) _wc_ranged)
    (else
      (`SceneComponent.SetVisibility` (`self.WC_Melee`) true true)
      (`SceneComponent.SetVisibility` (`self.WC_Ranged`) false true))))

(fn `IsInteractable`
  (returns (isInteractable :type Boolean))
  (return false))

(fn `RagDollOnHit`
  (bind _mesh (`self.Mesh`))
  (`PrimitiveComponent.SetCollisionEnabled` _mesh "QueryAndPhysics")
  (`PrimitiveComponent.SetSimulatePhysics` _mesh true)
  (`SkeletalMeshComponent.SetPhysicsBlendWeight` _mesh 1.0)
  (set `self.isDead` true)
  (`self.SetLifeSpan` 2.0))

(fn `UserConstructionScript`
  (`self.Set Enemy Type`))